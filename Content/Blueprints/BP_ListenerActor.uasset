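; BP_ListenerActor is an actor that listens for a value change on a target actor and destroys itself when one is reported.
; On BeginPlay, with authority only, it validates TargetActor and passes its capture value interface to the CaptureValueChangeAsync task.
; The task's Complete delegate triggers destruction if NewValueChanged is true.
; Debug strings report listening, destruction, failed capture or an invalid target.
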(event `self.ReceiveBeginPlay`
  (`self.InitializeCaptureValue`))

(event `InitializeCaptureValue`
  ;[1 0.3633 0.4692] Initialize Async Task to capture target value
  (`/Engine/EditorBlueprintResources/ActorMacros.Switch Has Authority`
    (:`Authority`
      (bind _targetactor (`self.TargetActor`)
        (:`then`
          (bind (_targetactor_2 _bnewvaluechanged) (`AsyncCaptureValueChange.CaptureValueChangeAsync` (`TargetActor.GetCaptureValueInterface` _targetactor))
            (:`then`
              (`KismetSystemLibrary.PrintString` "Listening Target Actor"))
            (:`OnCompleteDelegate`
              (if _bnewvaluechanged
                (`KismetSystemLibrary.PrintString` "Destroying Listener Actor" true true (struct :`G` 0.66 :`B` 1.0 :`A` 1.0) 5.0)
                (`self.K2_DestroyActor`)))
            (:`OnFailDelegate`
              (`KismetSystemLibrary.PrintString` "Fail to capture a value change"))))
        (:`else`
          (`KismetSystemLibrary.PrintString` "Actor was removed"))))))

(fn `UserConstructionScript`)