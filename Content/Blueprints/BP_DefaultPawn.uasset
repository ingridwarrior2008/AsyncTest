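; BP_DefaultPawn is a pawn that lets player input change an async destroy value on the level's BP_TargetActor.
; BeginPlay caches the target actor and adds the IM_Context Enhanced Input mapping for player controller 0.
; IA_ChangeVariable passes true through a server-named event, which calls SetNewAsyncDestroyValue on the target, with debug prints marking the call and the change.
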(event `self.ReceiveBeginPlay`
  (bind _returnvalue (pcsubsystem `EnhancedInputLocalPlayerSubsystem` (`GameplayStatics.GetPlayerController` 0)))
  (bind _returnvalue_2 (`GameplayStatics.GetActorOfClass` "/Game/Blueprints/BP_TargetActor.BP_TargetActor_C"))
  (set `self.TargetActor` _returnvalue_2)
  ;[1 0.2673 0.1173] Setup Input
  (`/Engine/EditorBlueprintResources/StandardMacros.IsValid` _returnvalue
    (:`Is Valid`
      (`EnhancedInputSubsystemInterface.AddMappingContext` _returnvalue "/Game/Input/IM_Context.IM_Context" 0 (struct)))))

(event `EnhancedInput|/Game/Input/IA_ChangeVariable`
  (params (ActionValue :type Boolean) (ElapsedSeconds :type "Float (double-precision)") (TriggeredSeconds :type "Float (double-precision)") (InputAction :type "InputAction Object Reference" :default "/Game/Input/IA_ChangeVariable.IA_ChangeVariable"))
  ;[0.2812 0.2535 1] Change Value
  (:`Triggered`
    (`self.Server_SetNewAsyncDestroyValue` true)
    (`KismetSystemLibrary.PrintString` "Call Value")))

(event `Server_SetNewAsyncDestroyValue`
  (params (bNewValue :type Boolean))
  ;[0.2812 0.2535 1] Change Value
  (`TargetActor.SetNewAsyncDestroyValue` (`self.TargetActor`) bNewValue)
  (`KismetSystemLibrary.PrintString` "Cahnged Value"))

(fn `UserConstructionScript`)